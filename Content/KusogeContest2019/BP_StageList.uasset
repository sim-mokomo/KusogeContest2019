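; BP_StageList builds a stage as a chain of BP_StageSection child actors.
; Its construction script loops by SectionNum, adding each child actor component at the joint position of the last SectionList entry and appending the new section to that list.
; The script stops if a child fails the BP_StageSection cast, and the Initialize event is empty.
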(event `Initialize`)

(fn `UserConstructionScript`
  (bind _sectionlist (`self.SectionList`))
  (for _ (range (+ (`self.SectionNum`) 1))
    (bind _returnvalue (`AddComponent|NODE_AddChildActorComponent-0` :`RelativeTransform` (`KismetMathLibrary.Conv_VectorToTransform` (`/Game/KusogeContest2019/BP_StageSection.GetJointPos` (`|GetArrayItem` _sectionlist (`KismetArrayLibrary.Array_LastIndex` _sectionlist))))))
    (bind _asbp_stage_section (cast `/Game/KusogeContest2019/BP_StageSection` (`ChildActorComponent.ChildActor` _returnvalue)))
    (`KismetArrayLibrary.Array_Add` (`self.SectionList`) _asbp_stage_section)))