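; Player Blueprint for a mouse-flick movement game on the YZ plane.
; A right-mouse drag longer than a threshold line-traces in the flick direction and stores the hit point, offset along Y by the surface normal, as the target.
; Tick lerps the actor to that target without sweeping, while a timeline plays a spring scale animation on the mesh.
; Debug prints and trace drawing remain active.
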(event `self.ReceiveTick`
  (params (DeltaSeconds :type "Float (single-precision)"))
  (bind _distmoveloc (`self.DistMoveLoc`))
  (if (> (`KismetMathLibrary.VSize` _distmoveloc) 0.0)
    (`self.K2_SetActorLocation` (`KismetMathLibrary.VLerp` (`self.K2_GetActorLocation`) _distmoveloc (`self.MoveLerpSpeed`)))))

(event `SpringAnim`
  (bind (_direction _springstartscale) (`Timeline|SpringAnimTimeLine` :!via `PlayFromStart`)
    (:`Update`
      (`SceneComponent.SetWorldScale3D` (`self.PlayerMesh`) _springstartscale))))

(event `self.ReceiveBeginPlay`
  (bind _returnvalue (`GameplayStatics.GetPlayerController` 0))
  (set `PlayerController.bShowMouseCursor` true _returnvalue)
  (`self.EnableInput` _returnvalue)
  (`TimelineComponent.SetPlayRate` (`self.SpringAnimTimeLine`) (`self.SpringAnimSpeedRate`)))

(event `Key|RightMouseButton`
  (params (Key :type "Key Structure"))
  (bind _returnvalue (`self.K2_GetActorLocation`))
  (bind _returnvalue_2 (- (`self.EndDragPos`) (`self.StartDragPos`)))
  (bind _returnvalue_3 (`KismetMathLibrary.VSize2D` _returnvalue_2))
  (bind (_x _y) (`KismetMathLibrary.BreakVector2D` (* (`KismetMathLibrary.Normal2D` _returnvalue_2) 1000.0)))
  (:`Pressed`
    (bind _returnvalue_4 (`WidgetLayoutLibrary.GetMousePositionOnViewport`))
    (set `self.StartDragPos` _returnvalue_4))
  (:`Released`
    (bind _returnvalue_5 (`WidgetLayoutLibrary.GetMousePositionOnViewport`))
    (set `self.EndDragPos` _returnvalue_5)
    (`KismetSystemLibrary.PrintString` (`KismetStringLibrary.Conv_DoubleToString` _returnvalue_3))
    (if (>= _returnvalue_3 (`self.FlickThrethhold`))
      (bind _outhit (`KismetSystemLibrary.LineTraceSingle` :`Start` _returnvalue :`End` (+ _returnvalue (`KismetMathLibrary.MakeVector` 0.0 _x (* _y -1.0))) :`TraceChannel` "TraceTypeQuery1" :`DrawDebugType` "ForDuration"))
      (bind (_bblockinghit _binitialoverlap _time _distance _location _impactpoint _normal) (`GameplayStatics.BreakHitResult` _outhit))
      (bind _returnvalue_6 (`KismetMathLibrary.Dot_VectorVector` _normal (`KismetMathLibrary.GetRightVector` (struct))))
      (`KismetSystemLibrary.PrintString` (`KismetStringLibrary.Conv_DoubleToString` _returnvalue_6))
      (set `self.DistMoveLoc` (+ _location (* (0.0 26.0 0.0) _returnvalue_6)))
      (`self.SpringAnim`))))

(fn `UserConstructionScript`)