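; A cube actor that rolls and hops between grid panels, tracking its current panel and X/Y coordinates with a debug position label.
; SetPos records the previous and target panels, snaps on first placement, yaws the cube toward the target and, unless Only is set, fires OnSetPos.
; That event plays a step sound and the JumpAnim timeline, combining position lerp, height offset, squash-stretch and pitch roll, then calls OnEndMove.
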(event `self.ReceiveBeginPlay`
  (add `self.OnSetPos` (delegate `OnSetPosEvent`))
  (`TimelineComponent.SetPlayRate` (`self.JumpAnim`) (`self.AnimSpeedRatio`)))

(event `OnSetPosEvent`
  (bind (_prerotate_roll _prerotate_pitch _prerotate_yaw) (`KismetMathLibrary.BreakRotator` (`self.PreRotate`)))
  (`GameplayStatics.PlaySound2D` "/Game/KusogeContest2019/OutSource/SW_CubeStep.SW_CubeStep" 1.0 1.0 0.0 null null)
  (set `self.PreRotate` (`SceneComponent.RelativeRotation` (`self.Scene`)))
  (bind (_direction _animratio _animheightvalue _scalez _rotx) (`Timeline|JumpAnim` :!via `PlayFromStart`)
    (:`Update`
      (`self.K2_SetActorLocation` (`KismetMathLibrary.MakeVector` (.x (`KismetMathLibrary.VLerp` (`self.PreLoc`) (`self.GetPanelLoc` (`self.CurrentPanel`)) _animratio)) (.y (`KismetMathLibrary.VLerp` (`self.PreLoc`) (`self.GetPanelLoc` (`self.CurrentPanel`)) _animratio)) (+ (.z (`KismetMathLibrary.VLerp` (`self.PreLoc`) (`self.GetPanelLoc` (`self.CurrentPanel`)) _animratio)) _animheightvalue)))
      (`SceneComponent.SetRelativeScale3D` (`self.CubeMesh`) (`KismetMathLibrary.MakeVector` 1.0 1.0 _scalez))
      (`SceneComponent.K2_SetRelativeRotation` (`self.Scene`) (`KismetMathLibrary.MakeRotator` _prerotate_roll _rotx _prerotate_yaw) false false))
    (:`Finished`
      (`self.OnEndMove`))))

(fn `GetPanelLoc`
  (params (Panel :type "Actor Object Reference"))
  (returns (PanelLoc :type "Vector Structure"))
  (return (+ (`self.K2_GetActorLocation` Panel) (0.0 0.0 25.0))))

(fn `GetPos`
  (returns (PosX :type Integer) (PosY :type Integer))
  (return (`self.PosX`) (`self.PosY`)))

(fn `SetPos`
  (params (Panel :type "/Game/KusogeContest2019/BP_StagePanel Object Reference") (Only :type Boolean))
  (bind _returnvalue (`KismetMathLibrary.GetForwardVector` (struct)))
  (bind _currentpanel (`self.CurrentPanel`))
  (bind _returnvalue_2 (`KismetMathLibrary.Normal` (- (`KismetMathLibrary.MakeVector` (.x (`self.GetPanelLoc` (`self.CurrentPanel`))) (.y (`self.GetPanelLoc` (`self.CurrentPanel`)))) (`KismetMathLibrary.MakeVector` (.x (`SceneComponent.K2_GetComponentLocation` (`self.CubeMesh`))) (.y (`SceneComponent.K2_GetComponentLocation` (`self.CubeMesh`)))))))
  (bind _returnvalue_3 (`KismetMathLibrary.DegAcos` (`KismetMathLibrary.Dot_VectorVector` _returnvalue _returnvalue_2)))
  (`|ExecutionSequence`
    (:`then_0`
      (`/Engine/EditorBlueprintResources/StandardMacros.IsValid` _currentpanel
        (:`Is Valid`
          (set `self.PreLoc` (`self.GetPanelLoc` _currentpanel)))
        (:`Is Not Valid`
          (`self.K2_SetActorLocation` (`self.GetPanelLoc` Panel)))))
    (:`then_1`
      (bind _output_get (set `self.CurrentPanel` Panel))
      (bind (_posx _posy) (`/Game/KusogeContest2019/BP_StagePanel.GetPos` _output_get))
      (set `self.PosX` _posx)
      (set `self.PosY` _posy)
      (`self.UpdateDebugPos`)
      (`SceneComponent.K2_SetWorldRotation` (`self.Scene`) (`KismetMathLibrary.MakeRotator` 0.0 0.0 (* _returnvalue_3 (select `bool` (<= _returnvalue_3 90.0) :`false` 1.0 :`true` (`KismetMathLibrary.SignOfFloat` (.z (`KismetMathLibrary.Cross_VectorVector` _returnvalue _returnvalue_2)))))) false false)
      (if (not Only)
        (`self.OnSetPos`)))))

(fn `UpdateDebugPos`
  (`TextRenderComponent.K2_SetText` (`self.DebugPos`) (`KismetTextLibrary.Conv_StringToText` (`KismetStringLibrary.Concat_StrStr` "(" (`KismetStringLibrary.Conv_IntToString` (`self.PosX`)) "," (`KismetStringLibrary.Conv_IntToString` (`self.PosY`)) ")"))))

(fn `UserConstructionScript`)