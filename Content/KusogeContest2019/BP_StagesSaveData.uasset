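; BP_StagesSaveData holds per-stage save data, including rank, for the KusogeContest2019 game.
; A StageDatas map keys stage save structs by Id, and Add inserts or overwrites an entry.
; GetStageData returns the stored entry, or builds a default struct with that Id and a fixed rank when none exists.
; GetSlotName supplies the constant save slot name.
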(fn `Add`
  (params (SaveData :type "/Game/KusogeContest2019/S_StageSaveData Structure (by ref)"))
  (`BlueprintMapLibrary.Map_Add` (`self.StageDatas`) (`.id_4_2C5496F14EB8CFED382BDDB0E8B558AE` (break `/Game/KusogeContest2019/S_StageSaveData` SaveData)) SaveData))

(fn `GetSlotName`
  (returns (SlotName :type String))
  (return "StagesSaveData"))

(fn `GetStageData`
  (params (StageId :type Integer))
  (returns (StageData :type "/Game/KusogeContest2019/S_StageSaveData Structure"))
  (bind (_value _returnvalue) (`BlueprintMapLibrary.Map_Find` (`self.StageDatas`) StageId))
  (if _returnvalue
    (return _value)
    (else
      (return (make `/Game/KusogeContest2019/S_StageSaveData` StageId "NewEnumerator3")))))