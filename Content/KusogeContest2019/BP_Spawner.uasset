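; BP_Spawner is an actor that spawns BP_Ball actors at random points inside a box-shaped spawn area.
; The construction script sizes the SpawnArea box from the SpawnAreaSize variable.
; The RandomSpawn event offsets the box's world location by a random amount within that extent on each axis, then spawns a scaled-down ball with a short, fixed life span.
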(event `RandomSpawn`
  (bind (_spawnareasize_x _spawnareasize_y _spawnareasize_z) (`KismetMathLibrary.BreakVector` (`self.SpawnAreaSize`)))
  (bind _returnvalue (`|SpawnActorFromClass` "/Game/KusogeContest2019/BP_Ball.BP_Ball_C" (`KismetMathLibrary.MakeTransform` (`KismetMathLibrary.MakeVector` (+ (.x (`SceneComponent.K2_GetComponentLocation` (`self.SpawnArea`))) (`KismetMathLibrary.RandomFloatInRange` (* _spawnareasize_x -1.0) _spawnareasize_x)) (+ (.y (`SceneComponent.K2_GetComponentLocation` (`self.SpawnArea`))) (`KismetMathLibrary.RandomFloatInRange` (* _spawnareasize_y -1.0) _spawnareasize_y)) (+ (.z (`SceneComponent.K2_GetComponentLocation` (`self.SpawnArea`))) (`KismetMathLibrary.RandomFloatInRange` (* _spawnareasize_z -1.0) _spawnareasize_z))) (struct) (0.3 0.3 0.3)) "Undefined" "OverrideRootScale" null null))
  (`self.SetLifeSpan` _returnvalue 8.0))

(fn `UserConstructionScript`
  (`BoxComponent.SetBoxExtent` (`self.SpawnArea`) (`self.SpawnAreaSize`) true))