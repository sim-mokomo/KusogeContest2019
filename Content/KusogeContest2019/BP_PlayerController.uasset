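; Player controller for a mouse-driven game where the player places and angles spring boards.
; It shows the cursor and, on left click, spawns a BP_SpringBoard where the deprojected mouse ray hits the vertical X=0 plane.
; While the button is held, vertical drag distance from the press point rotates that board around the X axis, clamped to 90 degrees either way.
; Releasing the button ends control of the board.
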(event `self.ReceiveBeginPlay`
  (set `self.bShowMouseCursor` true))

(event `Key|LeftMouseButton`
  (params (Key :type "Key Structure"))
  (bind (_worldlocation _worlddirection) (`self.DeprojectMousePositionToWorld`))
  (:`Pressed`
    (bind _returnvalue (`|SpawnActorFromClass` "/Game/KusogeContest2019/BP_SpringBoard.BP_SpringBoard_C" (`KismetMathLibrary.MakeTransform` (`.Intersection` (`KismetMathLibrary.LinePlaneIntersection_OriginNormal` _worldlocation (+ _worldlocation (* _worlddirection 10000.0)) (0.0 0.0 0.0) (-1.0 0.0 0.0)))) "Undefined" "OverrideRootScale" null null))
    (set `self.CurrentControllSpringBoard` _returnvalue)
    (set `self.StartMousePosY` (`.LocationY` (`self.GetMousePosition`))))
  (:`Released`
    (set `self.CurrentControllSpringBoard` null)))

(event `self.ReceiveTick`
  (params (DeltaSeconds :type "Float (single-precision)"))
  (bind _returnvalue (- (`self.CurrentMousePosY`) (`self.StartMousePosY`)))
  (if (`self.IsInputKeyDown` "LeftMouseButton")
    (`/Engine/EditorBlueprintResources/StandardMacros.IsValid` (`self.CurrentControllSpringBoard`)
      (:`Is Valid`
        (set `self.CurrentMousePosY` (`.LocationY` (`self.GetMousePosition`)))
        (`self.K2_SetActorRotation` (`self.CurrentControllSpringBoard`) (`KismetMathLibrary.RotatorFromAxisAndAngle` (1.0 0.0 0.0) (* (`KismetMathLibrary.Lerp` 0.0 90.0 (`KismetMathLibrary.FMin` (/ (`KismetMathLibrary.Abs` _returnvalue) 90.0) 1.0)) (`KismetMathLibrary.SignOfFloat` _returnvalue))) false)))))

(fn `UserConstructionScript`)