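; BP_StagePanel is a stage tile that holds a position, type and jump number, with its color looked up from the number in ColorTable.
; It tints a dynamic material and scales up via a timeline on BeginPlay.
; ChangeNextColor cycles the number, recolors the panel and spawns a tinted aura, which Finalize destroys; Explosion spawns a matching splash.
; Getters expose panel state and mesh size, and construction writes the coordinates to debug text.
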(event `Finalize`
  (bind _auravfx (`self.AuraVfx`))
  (`/Engine/EditorBlueprintResources/StandardMacros.IsValid` _auravfx
    (:`Is Valid`
      (`ActorComponent.K2_DestroyComponent` _auravfx))))

(event `Explosion`
  (bind _returnvalue (`GameplayStatics.SpawnEmitterAtLocation` "/Game/KusogeContest2019/P_Sprash.P_Sprash" (`self.K2_GetActorLocation`)))
  (`ParticleSystemComponent.SetVectorParameter` _returnvalue "BaseColor" (`KismetMathLibrary.Conv_LinearColorToVector` (`BlueprintMapLibrary.Map_Find` (`self.ColorTable`) (`self.JumpNumber`)))))

(event `self.ReceiveBeginPlay`
  (`self.SetPanelColor` (`self.JumpNumber`))
  (`TimelineComponent.SetPlayRate` (`self.ShowAnim`) (`self.ShowAnimRatio`))
  (bind (_direction _showanimratio) (`Timeline|ShowAnim`)
    (:`Update`
      (`SceneComponent.SetWorldScale3D` (`self.PanelMesh`) (`KismetMathLibrary.VLerp` (0.0 0.0 0.0) (1.0 1.0 1.0) _showanimratio)))))

(event `ChangeNextColor`
  (bind _result (`/Engine/EditorBlueprintResources/StandardMacros.IncrementInt` (`self.JumpNumber`))
    (:`  `
      (if (> _result (`BlueprintMapLibrary.Map_Length` (`self.ColorTable`)))
        (set `self.JumpNumber` 1))
      (`self.SetPanelColor` (`self.JumpNumber`))
      ;[1 1 1] オーラエフェクト再生
      (bind _returnvalue (`GameplayStatics.SpawnEmitterAtLocation` "/Game/KusogeContest2019/P_EnergyWall.P_EnergyWall" (+ (`self.K2_GetActorLocation`) (0.0 0.0 100.0))))
      (bind _output_get (set `self.AuraVfx` _returnvalue))
      (`ParticleSystemComponent.SetVectorParameter` _output_get "BaseColor" (`KismetMathLibrary.Conv_LinearColorToVector` (`BlueprintMapLibrary.Map_Find` (`self.ColorTable`) (`self.JumpNumber`)))))))

(fn `GetColor`
  (returns (Value :type "LinearColor Structure"))
  (return (`BlueprintMapLibrary.Map_Find` (`self.ColorTable`) (`self.JumpNumber`))))

(fn `GetJumpNumber`
  (returns (JumpNumber :type Integer))
  (return (`self.JumpNumber`)))

(fn `GetMeshHeight`
  (returns (ReturnValue :type "Float (double-precision)"))
  (return (* (.y (`.BoxExtent` (`KismetSystemLibrary.GetComponentBounds` (`self.PanelMesh`)))) 2.0)))

(fn `GetMeshWidth`
  (returns (Width :type "Float (double-precision)"))
  (return (* (.x (`.BoxExtent` (`KismetSystemLibrary.GetComponentBounds` (`self.PanelMesh`)))) 2.0)))

(fn `GetPos`
  (returns (PosX :type Integer) (PosY :type Integer))
  (return (`self.PosX`) (`self.PosY`)))

(fn `GetType`
  (returns (Type :type "/Game/KusogeContest2019/E_Panel Enum"))
  (return (`self.Type`)))

(fn `SetPanelColor`
  (params (Number :type Integer))
  (bind _bodydmi (`self.BodyDMI`))
  (bind (_value _returnvalue) (`BlueprintMapLibrary.Map_Find` (`self.ColorTable`) Number))
  (if _returnvalue
    (`MaterialInstanceDynamic.SetVectorParameterValue` _bodydmi "BaseColor" _value)
    (else
      (`KismetSystemLibrary.PrintString` (`KismetStringLibrary.Conv_IntToString` Number))
      (`MaterialInstanceDynamic.SetVectorParameterValue` :`self` _bodydmi :`ParameterName` "BaseColor")))
  (set `self.JumpNumber` Number))

(fn `UpdateDebugPos`
  (`TextRenderComponent.K2_SetText` (`self.DebugPos`) (`KismetTextLibrary.Conv_StringToText` (`KismetStringLibrary.Concat_StrStr` "(" (`KismetStringLibrary.Conv_IntToString` (`self.PosX`)) "," (`KismetStringLibrary.Conv_IntToString` (`self.PosY`)) ")"))))

(fn `UserConstructionScript`
  (bind _returnvalue (`PrimitiveComponent.CreateDynamicMaterialInstance` (`self.PanelMesh`) 0 "/Game/KusogeContest2019/M_StagePanel_Inst.M_StagePanel_Inst" "None"))
  (set `self.BodyDMI` _returnvalue)
  (`self.UpdateDebugPos`))