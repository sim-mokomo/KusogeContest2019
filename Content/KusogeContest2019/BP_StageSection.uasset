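; BP_StageSection is a stage section actor with left and right wall meshes and a joint component.
; The construction script places the two walls symmetrically along the local X axis using WallBetweenOffset, so the gap is tunable per instance.
; GetJointPos returns the world location of SectionJoint, apparently as an attachment point for chaining sections, and the event graph holds no active logic.
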(fn `GetJointPos`
  (returns (JointPos :type "Vector Structure"))
  (return (`SceneComponent.K2_GetComponentLocation` (`self.SectionJoint`))))

(fn `UserConstructionScript`
  (bind _wallbetweenoffset (`self.WallBetweenOffset`))
  (`SceneComponent.K2_SetRelativeLocation` (`self.RightWallMesh`) (`KismetMathLibrary.MakeVector` _wallbetweenoffset) false false)
  (`SceneComponent.K2_SetRelativeLocation` (`self.LeftWallMesh`) (`KismetMathLibrary.MakeVector` (* _wallbetweenoffset -1.0)) false false))