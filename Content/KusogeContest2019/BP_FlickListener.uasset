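; BP_FlickListener is an actor that detects mouse flick gestures, currently only printing their direction.
; It enables input and shows the cursor, records Y-inverted mouse positions on left button press and release, then prints the normalized difference.
; An unfinished, unused ConvertToFlickDirection function begins a four-sector angle test against the rotated actor up vector, but its branch does nothing and its enum return is disconnected.
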(event `self.ReceiveBeginPlay`
  (bind _returnvalue (`GameplayStatics.GetPlayerController` 0))
  (`self.EnableInput` _returnvalue)
  (set `PlayerController.bShowMouseCursor` true _returnvalue))

(event `Key|LeftMouseButton`
  (params (Key :type "Key Structure"))
  (bind (_locationx _locationy) (`PlayerController.GetMousePosition` (`GameplayStatics.GetPlayerController` 0)))
  (bind _returnvalue (`KismetMathLibrary.MakeVector2D` _locationx (* _locationy -1.0)))
  (:`Pressed`
    (set `self.StartMousePos` _returnvalue))
  (:`Released`
    (set `self.EndMousePos` _returnvalue)
    (`KismetSystemLibrary.PrintString` (`KismetStringLibrary.Conv_Vector2dToString` (`KismetMathLibrary.Normal2D` (- (`self.EndMousePos`) (`self.StartMousePos`)))))))

(fn `ConvertToFlickDirection`
  (params (Direction :type "Vector2D Structure"))
  (returns (FlickDirection :type "/Game/KusogeContest2019/E_FlickDirection Enum"))
  (bind _returnvalue (/ 360.0 4.0))
  (if (<= (`KismetMathLibrary.Acos` (`KismetMathLibrary.Dot_VectorVector` (`KismetMathLibrary.GreaterGreater_VectorRotator` (`self.GetActorUpVector`) (`KismetMathLibrary.MakeRotator` (* _returnvalue 0.5))) (`KismetMathLibrary.Conv_Vector2DToVector` Direction))) _returnvalue)
    _))

(fn `UserConstructionScript`)