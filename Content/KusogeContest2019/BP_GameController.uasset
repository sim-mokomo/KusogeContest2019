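; Game controller for a tile-board puzzle that handles player input and connects the StageBoard to the movable RoringBox.
; On BeginPlay it switches to the main camera, initializes the board from each StageConfig DataTable row, read as string columns, and places the box on the start panel.
; Arrow keys move the box one panel when the destination exists.
; Space advances the color of the panels StageBoard returns as round the box's panel.
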(event `self.ReceiveBeginPlay`
  (`self.EnableInput` (`GameplayStatics.GetPlayerController` 0))
  (`PlayerController.SetViewTargetWithBlend` (`GameplayStatics.GetPlayerController` 0) (`self.MainCamera`) 0.0 "VTBlend_Linear" 0.0 false)
  (bind _returnvalue (`DataTableFunctionLibrary.GetDataTableColumnAsString` "/Game/KusogeContest2019/StageConfig_-_シート1.StageConfig_-_シート1" "stage_datas"))
  (bind _returnvalue_2 (`DataTableFunctionLibrary.GetDataTableColumnAsString` "/Game/KusogeContest2019/StageConfig_-_シート1.StageConfig_-_シート1" "start_jump_power"))
  (for (_array_element _array_index) _returnvalue
    (`/Game/KusogeContest2019/BP_StageBoard.Initialize` (`self.StageBoard`) (make `/Game/KusogeContest2019/S_StageConfigRow` _array_index _array_element (`KismetStringLibrary.Conv_StringToInt` (`|GetArrayItem` _returnvalue_2 _array_index)))))
  (`/Game/KusogeContest2019/BP_RoringCube.SetPos` (`self.RoringBox`) (`/Game/KusogeContest2019/BP_StageBoard.GetStartPanel` (`self.StageBoard`))))

(event `Key|Right`
  (params (Key :type "Key Structure"))
  (:`Pressed`
    (`self.MoveCube` 1)))

(event `Key|Left`
  (params (Key :type "Key Structure"))
  (:`Pressed`
    (`self.MoveCube` -1)))

(event `Key|Up`
  (params (Key :type "Key Structure"))
  (:`Pressed`
    (`self.MoveCube` 0 1)))

(event `Key|Down`
  (params (Key :type "Key Structure"))
  (:`Pressed`
    (`self.MoveCube` 0 -1)))

(event `Key|SpaceBar`
  (params (Key :type "Key Structure"))
  (bind _stageboard (`self.StageBoard`))
  (bind (_posx _posy) (`/Game/KusogeContest2019/BP_RoringCube.GetPos` (`self.RoringBox`)))
  (:`Pressed`
    (bind _arroundpanels (`/Game/KusogeContest2019/BP_StageBoard.GetRoundPanels` _stageboard (`/Game/KusogeContest2019/BP_StageBoard.GetPanel` _stageboard _posx _posy)))
    (for _array_element _arroundpanels
      (`/Game/KusogeContest2019/BP_StagePanel.ChangeNextColor` _array_element))))

(fn `MoveCube`
  (params (DiffX :type Integer) (DiffY :type Integer))
  (bind _roringbox (`self.RoringBox`))
  (bind (_posx _posy) (`/Game/KusogeContest2019/BP_RoringCube.GetPos` _roringbox))
  (bind _panel (`/Game/KusogeContest2019/BP_StageBoard.GetPanel` (`self.StageBoard`) (+ _posx DiffX) (+ _posy DiffY)))
  (`/Engine/EditorBlueprintResources/StandardMacros.IsValid` _panel
    (:`Is Valid`
      (`/Game/KusogeContest2019/BP_RoringCube.SetPos` _roringbox _panel))))

(fn `UserConstructionScript`)