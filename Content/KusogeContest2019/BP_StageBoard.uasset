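; BP_StageBoard is the stage board actor that builds and tracks a grid of BP_StagePanel tiles from a stage config.
; Initialize parses the config's stage data string into rows and comma-separated jump numbers, spawning panels spaced by mesh size plus offsets.
; A jump number of zero marks the start panel, which is colored by StartJumpPower, and helpers look up panels by grid position.
; With ShowDebug on, the construction script previews a grid using child actor components.
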(event `Initialize`
  (params (StageConfig :type "/Game/KusogeContest2019/S_StageConfigRow Structure"))
  (`self.GeneratePanels` StageConfig))

(fn `ConvertPos2VecPos`
  (params (Pos :type Integer))
  (returns (X :type Integer) (Y :type Integer))
  (bind _maxwidth (`self.MaxWidth`))
  (return (mod Pos _maxwidth) (/ Pos _maxwidth)))

(fn `GeneratePanel`
  (params (PosX :type Integer) (PosY :type Integer) (JumpNumber :type Integer))
  (returns (GeneratedPanel :type "/Game/KusogeContest2019/BP_StagePanel Object Reference"))
  (bind _returnvalue (`|SpawnActorFromClass` "/Game/KusogeContest2019/BP_StagePanel.BP_StagePanel_C" (`KismetMathLibrary.MakeTransform` (0.0 0.0 0.0)) "Undefined" "OverrideRootScale" null (`self.JumpNumber2PanelType` JumpNumber) JumpNumber PosX PosY null))
  (`self.K2_SetActorLocation` _returnvalue (`self.GetSpawnPosByGridIndex` PosX PosY _returnvalue) false false)
  (return _returnvalue))

(fn `GeneratePanels`
  (params (Config :type "/Game/KusogeContest2019/S_StageConfigRow Structure (by ref)"))
  (bind (_id _stage_datas _start_jump_power) (break `/Game/KusogeContest2019/S_StageConfigRow` Config))
  (`KismetArrayLibrary.Array_Clear` (`self.StagePanels`))
  (set `self.Config` Config)
  (for (_array_element _array_index) (`KismetStringLibrary.ParseIntoArray` (`KismetSystemLibrary.MakeLiteralString` _stage_datas) " \n")
    (bind _returnvalue (`KismetSystemLibrary.MakeLiteralString` _array_element))
    (`KismetSystemLibrary.PrintString` _returnvalue true true (struct :`G` 0.230108 :`B` 1.0 :`A` 1.0))
    (set `self.MaxHeight` (`KismetMathLibrary.Max` (`self.MaxHeight`) _array_index))
    (for (_array_element_2 _array_index_2) (`KismetStringLibrary.ParseIntoArray` _returnvalue ",")
      (`KismetSystemLibrary.PrintString` _array_element_2 true true (struct :`R` 1.0 :`G` 0.086574 :`A` 1.0))
      (bind _generatedpanel (`self.GeneratePanel` _array_index_2 _array_index (`KismetStringLibrary.Conv_StringToInt` _array_element_2)))
      (`KismetArrayLibrary.Array_Add` (`self.StagePanels`) _generatedpanel)
      (set `self.MaxWidth` (`KismetMathLibrary.Max` (`self.MaxWidth`) _array_index_2))))
  (`/Game/KusogeContest2019/BP_StagePanel.SetPanelColor` (`self.GetStartPanel`) _start_jump_power))

(fn `GetPanel`
  (params (X :type Integer) (Y :type Integer))
  (returns (Panel :type "/Game/KusogeContest2019/BP_StagePanel Object Reference"))
  (for _array_element (`self.StagePanels`)
    (bind (_posx _posy) (`/Game/KusogeContest2019/BP_StagePanel.GetPos` _array_element))
    (if (and (== _posx X) (== _posy Y))
      (return _array_element))))

(fn `GetSpawnPosByGridIndex`
  (params (X :type Integer) (Y :type Integer) (Panel :type "/Game/KusogeContest2019/BP_StagePanel Object Reference"))
  (returns (ReturnValue :type "Vector Structure"))
  (return (+ (`self.K2_GetActorLocation`) (`KismetMathLibrary.MakeVector` (* Y (+ (`/Game/KusogeContest2019/BP_StagePanel.GetMeshWidth` Panel) (`self.SpawnOffsetX`))) (* X (+ (`/Game/KusogeContest2019/BP_StagePanel.GetMeshHeight` Panel) (`self.SpawnOffsetY`)))))))

(fn `GetStageDatas`
  (params (RowIndex :type Integer))
  (returns (RowDatas :type "Array of String"))
  (locals (RowData :type "Array of String"))
  (for (_array_element _array_index) (`KismetStringLibrary.ParseIntoArray` (`KismetSystemLibrary.MakeLiteralString` (`.stage_datas_5_5870FE534903F81B8D92D7B6A0474683` (break `/Game/KusogeContest2019/S_StageConfigRow` (`self.Config`)))) " \n")
    (if (== _array_index RowIndex)
      (for _array_element_2 (`KismetStringLibrary.ParseIntoArray` (`KismetSystemLibrary.MakeLiteralString` _array_element) ",")
        (`KismetArrayLibrary.Array_Add` (`local.RowData`) _array_element_2))
      (return (`local.RowData`)))))

(fn `GetStartPanel`
  (returns (StartPanel :type "/Game/KusogeContest2019/BP_StagePanel Object Reference"))
  (for _array_element (`self.StagePanels`)
    (if (`|EnumEquality` (`/Game/KusogeContest2019/BP_StagePanel.Type` _array_element) "NewEnumerator0")
      (return _array_element)))
  (`KismetSystemLibrary.PrintString` "Nothing Start Panel ")
  (return null))

(fn `JumpNumber2PanelType`
  (params (JumpNumber :type Integer))
  (returns (PanelType :type "/Game/KusogeContest2019/E_Panel Enum"))
  (`|ExecutionSequence`
    (:`then_0`
      (if (== JumpNumber 0)
        (return "NewEnumerator0")))
    (:`then_1`
      (return "NewEnumerator2"))))

(fn `UserConstructionScript`
  (if (`self.ShowDebug`)
    (for _index (range (+ (`self.DebugPanelNumY`) 1))
      (for _index_2 (range (+ (`self.DebugPanelNumX`) 1))
        (bind _returnvalue (`AddComponent|NODE_AddChildActorComponent-0`))
        (bind _asbp_stage_panel (cast `/Game/KusogeContest2019/BP_StagePanel` (`ChildActorComponent.ChildActor` _returnvalue)))
        (`SceneComponent.K2_SetWorldLocation` _returnvalue (`self.GetSpawnPosByGridIndex` _index_2 _index _asbp_stage_panel) false false)))))