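; Player character Blueprint that hops forward along a ballistic arc when its Spring event is called with a spring board.
; Spring targets a point offset in X from the board at the character's current height, with the offset set through Initialize.
; CalculateVelocity solves projectile launch velocity from gravity, distance and JumpAngle, feeding LaunchCharacter with full velocity override.
; SpringCollisiion hits only print a debug message.
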(event `Initialize`
  (params (DefaultHoppingDistOffset :type "Float (double-precision)"))
  (set `self.DefaultHoppingDistOffset` DefaultHoppingDistOffset))

(event `/Game/KusogeContest2019/BP_Springable.Spring`
  (params (springBoard :type "/Game/KusogeContest2019/BP_SpringBoard Object Reference"))
  (bind _returnvalue (`self.K2_GetActorLocation`))
  (`self.LaunchCharacter` (`self.CalculateVelocity` _returnvalue (`KismetMathLibrary.MakeVector` (+ (.x (`self.K2_GetActorLocation` springBoard)) (`self.DefaultHoppingDistOffset`)) (.y (`self.K2_GetActorLocation` springBoard)) (.z _returnvalue)) (`self.JumpAngle`)) true true))

(event `self.SpringCollisiion.OnComponentHit`
  (params (HitComponent :type "PrimitiveComponent Object Reference") (OtherActor :type "Actor Object Reference") (OtherComp :type "PrimitiveComponent Object Reference") (NormalImpulse :type "Vector Structure") (Hit :type "HitResult Structure (by ref)"))
  (`KismetSystemLibrary.PrintString` "HIT!!!!!!"))

(fn `CalculateVelocity`
  (params (startPos :type "Vector Structure") (distPos :type "Vector Structure") (angle :type "Float (double-precision)"))
  (returns (ShootVec :type "Vector Structure"))
  (bind _returnvalue (`KismetMathLibrary.DegreesToRadians` angle))
  (bind _returnvalue_2 (`KismetMathLibrary.Vector_Distance2D` startPos distPos))
  (bind _returnvalue_3 (* _returnvalue_2 (`KismetMathLibrary.Tan` _returnvalue)))
  (return (* (`KismetMathLibrary.Normal` (`KismetMathLibrary.MakeVector` (- (.x distPos) (.x startPos)) (- (.y distPos) (.y startPos)) _returnvalue_3)) (`KismetMathLibrary.Sqrt` (/ (* (* (`MovementComponent.GetGravityZ` (`self.CharacterMovement`)) -1.0) (`KismetMathLibrary.MultiplyMultiply_FloatFloat` _returnvalue_2 2.0)) (* (* 2.0 (`KismetMathLibrary.MultiplyMultiply_FloatFloat` (`KismetMathLibrary.Cos` _returnvalue) 2.0)) (+ _returnvalue_3 (- (.z distPos) (.z startPos)))))))))

(fn `UserConstructionScript`)